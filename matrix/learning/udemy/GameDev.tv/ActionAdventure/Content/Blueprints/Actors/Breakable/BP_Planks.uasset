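; BP_Planks is a breakable plank barrier with hit points and a text readout of its health.
; AnyDamage subtracts from HP and refreshes the PlankHP text.
; At zero or below, a DoOnce turns on physics for seven static meshes so the planks collapse.
; If the text component is valid, it is destroyed, and physics switches off after a short delay, freezing the debris.
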(event EventTick
  (params (DeltaSeconds :type Float%20%28single-precision%29)))

(event Game|Damage|EventAnyDamage
  (params (Damage :type Float%20%28single-precision%29) (DamageType :type Damage%20Type%20Object%20Reference) (InstigatedBy :type Controller%20Object%20Reference) (DamageCauser :type Actor%20Object%20Reference))
  (bind _plankhp (Variables|Default|GetPlankHP))
  (bind _plankhp_2 (Variables|Default|GetPlankHP))
  (Variables|Default|SetHP (- (Variables|Default|GetHP) Damage))
  (if (Utilities|IsValid _plankhp_2)
    (Rendering|Components|TextRender|SetText _plankhp_2 (Utilities|Text|ToText(String) (Utilities|String|Append (Variables|Default|GetHPText) (Utilities|String|ToString(Text) (Utilities|Text|ToText(Float) (Variables|Default|GetHP) "HalfToEven"))))))
  (if (<= (Variables|Default|GetHP) 0.0)
    (Utilities|FlowControl|DoOnce false
      (:Completed
        (Physics|SetSimulatePhysics (Variables|Debug|GetStaticMeshComponent) true)
        (if (Utilities|IsValid _plankhp)
          (Components|DestroyComponent _plankhp)
          (Utilities|FlowControl|Delay 4.0)
          (Physics|SetSimulatePhysics (Variables|Debug|GetStaticMeshComponent) false))))))

(fn ConstructionScript)