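; BP_QTE_Ledge is a trigger that runs a timed quick-time event at a ledge when BP_Savith_Player overlaps its box.
; On overlap it slows global time, shows the player's QTEX prompt and enables their QTE flag, then hides the prompt after a short delay.
; If QTESuccess is set, it plays the success level sequence and teleports the player to a hardcoded location, and normal time resumes either way.
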(event OnComponentBeginOverlap(Box)
  (params (OverlappedComponent :type Primitive%20Component%20Object%20Reference) (OtherActor :type Actor%20Object%20Reference) (OtherComp :type Primitive%20Component%20Object%20Reference) (OtherBodyIndex :type Integer) (bFromSweep :type Boolean) (SweepResult :type Hit%20Result%20Structure%20%28by%20ref%29))
  (bind _asbp_savith_player (Utilities|Casting|CastToBP_Savith_Player OtherActor))
  (Utilities|IsValid _asbp_savith_player
    (:Is%20Valid
      (Utilities|Time|SetGlobalTimeDilation 0.2)
      (Rendering|SetVisibility (Variables|/Game/Blueprints/Actors/Pawns/Character/BP_Savith_Player.BP_Savith_Player_C|GetQTE_X _asbp_savith_player) true false)
      (Variables|/Game/Blueprints/Actors/Pawns/Character/BP_Savith_Player.BP_Savith_Player_C|SetQTE? _asbp_savith_player true)
      (Utilities|FlowControl|Delay 0.75)
      (Rendering|SetVisibility (Variables|/Game/Blueprints/Actors/Pawns/Character/BP_Savith_Player.BP_Savith_Player_C|GetQTE_X _asbp_savith_player) false false)
      (if (Variables|/Game/Blueprints/Actors/Pawns/Character/BP_Savith_Player.BP_Savith_Player_C|GetQTESuccess? _asbp_savith_player)
        (bind _returnvalue (Sequencer|Player|CreateLevelSequencePlayer "/Game/Blueprints/Cinematics/QTE_Ledge_Success.QTE_Ledge_Success" (Utilities|Struct|MakeMovieSceneSequencePlaybackSettings false "(Value=0)" 0.75 0.0 false true true false true false false false)))
        (Sequencer|Player|Play _returnvalue :!class /Script/MovieScene.MovieSceneSequencePlayer)
        (Transformation|Teleport _asbp_savith_player "380.000000,1050.000000,1330.000000" "0, 0, 0"))
      (Utilities|Time|SetGlobalTimeDilation 1.0))))

(fn ConstructionScript)